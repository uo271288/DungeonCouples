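; BP_GoalChecker is a Blueprint that checks the level's win and lose conditions on Tick.
; When both PinkyGoal and BleueGoal are reached, it adds a new widget to the viewport, repeating each tick while that holds.
; A one-second Delay on Tick drives a Minutes/Seconds countdown, which adds a GameOver widget each time it fires at zero.
; Neither branch latches or stops the other.
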(event `self.ReceiveTick`
  (params (DeltaSeconds :type "Float (single-precision)"))
  (`|ExecutionSequence`
    (:`then_0`
      (if (and (`/Game/Blueprints/Goal/BP_PinkyGoal.Reached` (`self.PinkyGoal`)) (`/Game/Blueprints/Goal/BP_BleueGoal.Reached` (`self.BleueGoal`)))
        (bind _returnvalue (`|CreateWidget` "/Game/UI/Win.Win_C"))
        (`UserWidget.AddToViewport` _returnvalue 0)))
    (:`then_1`
      (`KismetSystemLibrary.Delay` 1.0)
      (if (== (`self.Seconds`) 0)
        (if (== (`self.Minutes`) 0)
          (bind _returnvalue_2 (`|CreateWidget` "/Game/UI/GameOver.GameOver_C"))
          (`UserWidget.AddToViewport` _returnvalue_2 0)
          (else
            (set `self.Seconds` 59)
            (`/Engine/EditorBlueprintResources/StandardMacros.DecrementInt` (`self.Minutes`))))
        (else
          (`/Engine/EditorBlueprintResources/StandardMacros.DecrementInt` (`self.Seconds`)))))))

(fn `UserConstructionScript`)