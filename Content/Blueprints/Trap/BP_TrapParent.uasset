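; BP_TrapParent is a base trap actor that ends the game when a matching player character touches it.
; On overlap it casts to BP_Character and compares the character's first actor tag to its own Tag value.
; A match plays the Pinky or Bleue scream at the character's location, then creates a GameOver widget and adds it to the viewport.
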(event `self.ReceiveActorBeginOverlap`
  (params (OtherActor :type "Actor Object Reference"))
  (bind _asbp_character (cast `/Game/Blueprints/BP_Character` OtherActor))
  (if (== (`|GetArrayItem` (`Actor.Tags` _asbp_character)) (`self.Tag`))
    (if (== (`self.Tag`) "Pinky")
      (bind _returnvalue (`self.K2_GetActorLocation` _asbp_character))
      (`GameplayStatics.PlaySoundAtLocation` "/Game/Sounds/Pinky_Scream.Pinky_Scream" _returnvalue (struct) 1.0 1.0 0.0 null null null)
      (else
        (`GameplayStatics.PlaySoundAtLocation` "/Game/Sounds/Bleue_Scream.Bleue_Scream" _returnvalue (struct) 1.0 1.0 0.0 null null null)))
    (bind _returnvalue_2 (`|CreateWidget` "/Game/UI/GameOver.GameOver_C"))
    (`UserWidget.AddToViewport` _returnvalue_2 0)))

(fn `UserConstructionScript`)