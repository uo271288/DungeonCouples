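; Parent Blueprint for a one-shot switch that spawns a platform tile when a matching character touches it.
; On overlap, it casts the actor to BP_Character and compares the character's first actor tag to its own Tag variable.
; A match swaps the Paper2D sprite, spawns the Tile class at PlatformTransform, plays the switch sound and sets Activated to block retriggering.
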(event `self.ReceiveActorBeginOverlap`
  (params (OtherActor :type "Actor Object Reference"))
  (bind _asbp_character (cast `/Game/Blueprints/BP_Character` OtherActor))
  (if (and (not (`self.Activated`)) (== (`|GetArrayItem` (`Actor.Tags` _asbp_character)) (`self.Tag`)))
    (`PaperSpriteComponent.SetSprite` (`self.PaperSprite`) (`self.Sprite`))
    (`|SpawnActorFromClass` (`self.Tile`) (`self.PlatformTransform`) "Undefined" "OverrideRootScale" null null)
    (set `self.Activated` true)
    (`GameplayStatics.PlaySoundAtLocation` "/Game/Sounds/Switch.Switch" (`self.K2_GetActorLocation`) (struct) 1.0 1.0 0.0 null null null)))

(fn `UserConstructionScript`)