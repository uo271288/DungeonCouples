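; BP_CollectableParent is a collectable pickup, named as a parent class, that awards a point to the character that touches it.
; On actor overlap it casts to BP_Character and compares that character's first actor tag with its own Tag value.
; On a match it increments the character's Points, plays the Collectable sound at its location and destroys itself.
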(event `self.ReceiveActorBeginOverlap`
  (params (OtherActor :type "Actor Object Reference"))
  (bind _asbp_character (cast `/Game/Blueprints/BP_Character` OtherActor))
  (if (== (`|GetArrayItem` (`Actor.Tags` _asbp_character)) (`self.Tag`))
    (`/Engine/EditorBlueprintResources/StandardMacros.IncrementInt` (`/Game/Blueprints/BP_Character.Points` _asbp_character)
      (:`  `
        (`GameplayStatics.PlaySoundAtLocation` "/Game/Sounds/Collectable.Collectable" (`self.K2_GetActorLocation`) (struct) 1.0 1.0 0.0 null null null)
        (`self.K2_DestroyActor`)))))

(fn `UserConstructionScript`)