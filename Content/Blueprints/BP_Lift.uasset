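; BP_Lift is a 2D lift that moves its Paper sprite back and forth between the relative origin and EndLocation.
; A timeline drives the position lerp, and on each finish it waits for Delay, then alternates LiftUp and LiftDown by toggling TestEndLocation.
; The construction script reuses TestEndLocation to preview the sprite at EndLocation.
; Nothing in this file makes the first LiftUp call.
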(event `LiftUp`
  (bind (_direction _driver) (`Timeline|LiftTimeline` :!via `PlayFromStart` :!label _label)
    (:`Update`
      (`SceneComponent.K2_SetRelativeLocation` (`self.PaperSprite`) (`KismetMathLibrary.VLerp` (0.0 0.0 0.0) (`self.EndLocation`) _driver) false false))
    (:`Finished`
      (`KismetSystemLibrary.Delay` (`self.Delay`))
      (if (`self.TestEndLocation`)
        (`self.LiftUp`)
        (else
          (`self.LiftDown`)))
      (set `self.TestEndLocation` (not (`self.TestEndLocation`))))))

(event `LiftDown`
  (goto _label :!via `ReverseFromEnd`))

(fn `UserConstructionScript`
  (`SceneComponent.K2_SetRelativeLocation` (`self.PaperSprite`) (`KismetMathLibrary.SelectVector` (`self.EndLocation`) (`SceneComponent.RelativeLocation` (`self.PaperSprite`)) (`self.TestEndLocation`)) false false))